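; Player Blueprint with camera-relative movement and a card hand, drawing on a deck of placeholder Fire cards with random mana costs.
; BeginPlay creates hand and HUD widgets, then updates stats, appends forty cards to the deck and fills the five-card hand.
; Number keys select a card unless quick cast is on, and F tries to use it.
; Z and X lower health or mana, then rerun that same stats-and-deck chain.
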(event `InputAxis|MoveForward`
  (params (AxisValue :type "Float (single-precision)"))
  (`self.AddMovementInput` (`SceneComponent.GetForwardVector` (`self.CameraBoom`)) AxisValue))

(event `Key|Z`
  (params (Key :type "Key Structure"))
  (:`Pressed`
    (set `self.Health` (- (`self.Health`) 10.0))
    (`/Game/UI/BP_UI/W_GameHud.UpdateStats` (`self.MainHUD_Ref`) (`self.Health`) (`self.MaxHealth`) (`self.Mana`) (`self.MaxMana`) :!label _label)
    (`self.InitDeck`)
    (for _ (range 1 6)
      (`self.DrawCard`))))

(event `Key|X`
  (params (Key :type "Key Structure"))
  (:`Pressed`
    (set `self.Mana` (- (`self.Mana`) 10.0))
    (goto _label)))

(event `InputAxis|MoveRight`
  (params (AxisValue :type "Float (single-precision)"))
  (`self.AddMovementInput` (`SceneComponent.GetRightVector` (`self.CameraBoom`)) AxisValue))

(event `self.ReceiveBeginPlay`
  (bind _returnvalue (`|CreateWidget` "/Game/UI/BP_UI/W_Hand.W_Hand_C"))
  (set `self.HandRef` _returnvalue)
  (`UserWidget.AddToViewport` _returnvalue 0)
  (bind _returnvalue_2 (`|CreateWidget` "/Game/UI/BP_UI/W_GameHud.W_GameHud_C"))
  (`UserWidget.AddToViewport` _returnvalue_2 0)
  (set `self.MainHUD_Ref` _returnvalue_2)
  (goto _label))

(event `Key|F`
  (params (Key :type "Key Structure"))
  (:`Pressed`
    (bind _asw_card (cast `/Game/UI/BP_UI/W_Card` (`PanelWidget.GetChildAt` (`/Game/UI/BP_UI/W_Hand.HandBox` (`self.HandRef`)) (`self.SelecredCardIndex`))))
    (`/Game/UI/BP_UI/W_Card.TryToUseCard` _asw_card)))

(event `Key|One`
  (params (Key :type "Key Structure"))
  (:`Pressed`
    (if (not (`self.bIsQuickCast`))
      (`self.SelectedSlot` 0))))

(event `Key|Two`
  (params (Key :type "Key Structure"))
  (:`Pressed`
    (if (not (`self.bIsQuickCast`))
      (`self.SelectedSlot` 1))))

(event `Key|Three`
  (params (Key :type "Key Structure"))
  (:`Pressed`
    (if (not (`self.bIsQuickCast`))
      (`self.SelectedSlot` 2))))

(event `Key|Four`
  (params (Key :type "Key Structure"))
  (:`Pressed`
    (if (not (`self.bIsQuickCast`))
      (`self.SelectedSlot` 3))))

(event `Key|Five`
  (params (Key :type "Key Structure"))
  (:`Pressed`
    (if (not (`self.bIsQuickCast`))
      (`self.SelectedSlot` 4))))

(fn `DrawCard`
  (if (> (`KismetArrayLibrary.Array_Length` (`self.Deck`)) 0)
    (if (< (`PanelWidget.GetChildrenCount` (`/Game/UI/BP_UI/W_Hand.HandBox` (`self.HandRef`))) 5)
      (bind _returnvalue (`|CreateWidget` "/Game/UI/BP_UI/W_Card.W_Card_C" (`GameplayStatics.GetPlayerController` 0) (struct) (`|GetArrayItem` (`self.Deck`))))
      (`PanelWidget.AddChild` (`/Game/UI/BP_UI/W_Hand.HandBox` (`self.HandRef`)) _returnvalue)
      (`KismetArrayLibrary.Array_Remove` (`self.Deck`)))))

(fn `InitDeck`
  (for _index (range 1 41)
    (`KismetArrayLibrary.Array_Add` (`self.Deck`) (make `CardData` (`KismetTextLibrary.Conv_StringToText` (`KismetStringLibrary.Concat_StrStr` "Card" (`KismetStringLibrary.Conv_IntToString` _index))) "" (`KismetMathLibrary.RandomIntegerInRange` 10 50) "/Game/Cards/Texture/fireball.fireball" "Common" "Fire"))))

(fn `SelectedSlot`
  (params (NewIndex :type Integer))
  (if (>= (`self.SelecredCardIndex`) 0)
    (bind _asw_card (cast `/Game/UI/BP_UI/W_Card` (`PanelWidget.GetChildAt` (`/Game/UI/BP_UI/W_Hand.HandBox` (`self.HandRef`)) (`self.SelecredCardIndex`))))
    (`/Game/UI/BP_UI/W_Card.SetSelected` _asw_card false))
  (set `self.SelecredCardIndex` (`local.NewIndex`))
  (bind _asw_card_2 (cast `/Game/UI/BP_UI/W_Card` (`PanelWidget.GetChildAt` (`/Game/UI/BP_UI/W_Hand.HandBox` (`self.HandRef`)) (`local.NewIndex`))))
  (`/Game/UI/BP_UI/W_Card.SetSelected` _asw_card_2 true))

(fn `UserConstructionScript`)